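; BP_CineCamera is a cinematic camera Blueprint that shows timed dialogue text on screen.
; It creates a WBP_Dialogue widget on BeginPlay and reuses it for each line.
; ShowDialogue sets the text, adds the widget to the viewport, plays BlendIn and starts a one-shot timer for the given seconds.
; The timer calls HideDialogue, which plays BlendOut and removes the widget when that animation finishes.
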(event Custom|ShowDialogue
  (params (Text :type Text) (Seconds :type Float%20%28double-precision%29))
  (bind _dialogueref (Variables|Default|GetDialogueRef))
  (Rendering|Components|TextRender|SetText (Variables|/Game/Items/Widgets/WBP_Dialogue.WBP_Dialogue_C|GetDialogueText _dialogueref) Text)
  (UserInterface|Viewport|AddtoViewport _dialogueref 0)
  (UserInterface|Animation|PlayAnimation _dialogueref (Variables|/Game/Items/Widgets/WBP_Dialogue.WBP_Dialogue_C|GetBlendIn _dialogueref) 0.0 1 "Forward" 1.0 false)
  (Utilities|Time|SetTimerbyEvent (delegate Custom|HideDialogue) Seconds))

(event Custom|HideDialogue
  (bind _dialogueref (Variables|Default|GetDialogueRef))
  (bind _blendout (Variables|/Game/Items/Widgets/WBP_Dialogue.WBP_Dialogue_C|GetBlendOut _dialogueref))
  (UserInterface|Animation|PlayAnimation _dialogueref _blendout 0.0 1 "Forward" 1.0 false)
  (Class|UserWidget|BindtoAnimationFinished _dialogueref _blendout (delegate Custom|RemoveFromParent)))

(event Custom|RemoveFromParent
  (Widget|RemovefromParent (Variables|Default|GetDialogueRef)))

(event EventBeginPlay
  (bind _returnvalue (UserInterface|CreateWidget "/Game/Items/Widgets/WBP_Dialogue.WBP_Dialogue_C"))
  (Variables|Default|SetDialogueRef _returnvalue))

(fn ConstructionScript)