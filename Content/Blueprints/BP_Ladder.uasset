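; BP_Ladder is a ladder actor that moves BP_Sophia into a preset pose when she enters its trigger box.
; On overlap it disables look and move input, then the CameraIn timeline lerps her location and control rotation from her actor transform to CameraAnimPosition.
; Input returns when the timeline finishes.
; No climbing logic is present, and end overlap only gets her camera component without using it.
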(event OnComponentBeginOverlap(Box)
  (params (OverlappedComponent :type Primitive%20Component%20Object%20Reference) (OtherActor :type Actor%20Object%20Reference) (OtherComp :type Primitive%20Component%20Object%20Reference) (OtherBodyIndex :type Integer) (bFromSweep :type Boolean) (SweepResult :type Hit%20Result%20Structure%20%28by%20ref%29))
  (bind _cameraanimposition (Variables|Default|GetCameraAnimPosition))
  (bind _returnvalue (Transformation|GetActorTransform _cameraanimposition))
  (bind _asbp_sophia (Utilities|Casting|CastToBP_Sophia OtherActor))
  (Variables|Default|SetPlayerLocation (Transformation|GetActorLocation _asbp_sophia))
  (Variables|Default|SetPlayerRotation (Transformation|GetActorRotation _asbp_sophia))
  (CallFunction|ToggleMovement true)
  (bind _alpha (Timeline|Camera%20In Play)
    (:Update
      (Transformation|SetActorLocation _asbp_sophia (Math|Vector|Lerp(Vector) (Variables|Default|GetPlayerLocation) (.location _returnvalue) _alpha) false false)
      (Pawn|SetControlRotation (Game|GetPlayerController 0) (Math|Rotator|Lerp(Rotator) (Variables|Default|GetPlayerRotation) (.rotation _returnvalue) _alpha)))
    (:Finished
      (CallFunction|ToggleMovement false))))

(event OnComponentEndOverlap(Box)
  (params (OverlappedComponent :type Primitive%20Component%20Object%20Reference) (OtherActor :type Actor%20Object%20Reference) (OtherComp :type Primitive%20Component%20Object%20Reference) (OtherBodyIndex :type Integer))
  (bind _asbp_sophia (Utilities|Casting|CastToBP_Sophia OtherActor))
  (Class|Sophia|GetCameraComponent _asbp_sophia))

(fn ConstructionScript)

(fn ToggleMovement
  (params (Status :type Boolean))
  (bind _returnvalue (Game|GetPlayerController 0))
  (Input|SetIgnoreLookInput _returnvalue Status)
  (Input|SetIgnoreMoveInput _returnvalue Status))