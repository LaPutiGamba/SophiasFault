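; BP_OptionsMesh is a clickable 3D options-menu entry that tilts its cube while selected and fades a spotlight on hover.
; BeginPlay enables mouse events, caches the WBP_OptionsMenu widget and selects option zero.
; Clicking deselects the current mesh, found by tag, then updates the widget's option and calls SelectOption.
; Tick drives a reversible rotation Timeline, with option 3 using a different axis, and lerps light intensity.
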(event OnClicked(Cube)
  (params (TouchedComponent :type Primitive%20Component%20Object%20Reference) (ButtonPressed :type Key%20Structure :default "None"))
  (bind _optionsmenucasted (Variables|Default|GetOptionsMenuCasted))
  (if (!= (Variables|/Game/Menu/WBP/WBP_OptionsMenu.WBP_OptionsMenu_C|GetnOption _optionsmenucasted) (Variables|Default|GetOption))
    (bind _outactors (Actor|GetAllActorsOfClasswithTag "BP_OptionsMesh_C" (Utilities|Array|Get(acopy) (Variables|Default|GetOptionTag) (Variables|/Game/Menu/WBP/WBP_OptionsMenu.WBP_OptionsMenu_C|GetnOption _optionsmenucasted))))
    (Variables|BP_OptionsMesh_C|SetIsSelected (Utilities|Array|Get(acopy) _outactors) false)
    (Variables|/Game/Menu/WBP/WBP_OptionsMenu.WBP_OptionsMenu_C|SetnOption _optionsmenucasted (Variables|Default|GetOption))
    (Default|SelectOption _optionsmenucasted)
    (Variables|Default|SetIsSelected true)))

(event OnBeginCursorOver(Cube)
  (params (TouchedComponent :type Primitive%20Component%20Object%20Reference))
  (Variables|Default|SetIsHover true))

(event OnEndCursorOver(Cube)
  (params (TouchedComponent :type Primitive%20Component%20Object%20Reference))
  (Variables|Default|SetIsHover false))

(event EventBeginPlay
  (bind _returnvalue (Game|GetPlayerController 0))
  (Variables|/Script/Engine.PlayerController|SetbEnableClickEvents _returnvalue true)
  (Variables|/Script/Engine.PlayerController|SetbEnableMouseOverEvents _returnvalue true)
  (bind _aswbp_options_menu (Utilities|Casting|CastToWBP_OptionsMenu (UserInterface|GetWidget (Variables|/Game/Menu/BP/BP_MenuOptions.BP_MenuOptions_C|GetWidget (Variables|Default|GetOptionsMenuRef)))))
  (bind _output_get (Variables|Default|SetOptionsMenuCasted _aswbp_options_menu))
  (Variables|/Game/Menu/WBP/WBP_OptionsMenu.WBP_OptionsMenu_C|SetnOption _output_get 0)
  (bind _outactors (Actor|GetAllActorsOfClasswithTag "BP_OptionsMesh_C" (Utilities|Array|Get(acopy) (Variables|Default|GetOptionTag) (Variables|/Game/Menu/WBP/WBP_OptionsMenu.WBP_OptionsMenu_C|GetnOption (Variables|Default|GetOptionsMenuCasted)))))
  (Variables|BP_OptionsMesh_C|SetIsSelected (Utilities|Array|Get(acopy) _outactors) true)
  (Variables|Default|SetInitialRotator (Variables|/Script/Engine.SceneComponent|GetRelativeRotation (Variables|Default|GetCube))))

(event EventTick
  (params (DeltaSeconds :type Float%20%28single-precision%29))
  (bind _cube (Variables|Default|GetCube))
  (bind _light (Variables|Default|GetLight))
  (bind _spotlightcomponent (Variables|/Script/Engine.SpotLight|GetSpotLightComponent _light))
  (Utilities|FlowControl|Sequence
    (:then_0
      (if (Variables|Default|GetIsSelected)
        (bind _newtrack_1 (Timeline|Timeline Play)
          (:Update
            (if (== (Variables|Default|GetOption) 3)
              (Transformation|SetRelativeRotation _cube (Math|Rotator|MakeRotator (Math|Float|Lerp 0.0 -45.0 _newtrack_1) 0.0 0.0) false false)
              (else
                (Transformation|SetRelativeRotation _cube (Math|Rotator|MakeRotator 0.0 (Math|Float|Lerp 0.0 45.0 _newtrack_1) 0.0) false false)))))
        (else
          (Timeline|Timeline Reverse))))
    (:then_1
      (if (Variables|Default|GetIsHover)
        (Rendering|Components|Light|SetIntensity _spotlightcomponent (Math|Float|Lerp (Variables|/Script/Engine.LightComponentBase|GetIntensity _spotlightcomponent) 15.0 0.1))
        (else
          (Rendering|Components|Light|SetIntensity _spotlightcomponent (Math|Float|Lerp (Variables|/Script/Engine.LightComponentBase|GetIntensity _spotlightcomponent) 0.0 0.1)))))))

(fn ConstructionScript)